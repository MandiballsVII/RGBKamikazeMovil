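; BP_BreakableRock is a rock actor that is destroyed when the player touches it while in one specific color state.
; On BeginPlay it casts player character 0 to BP_Player and stores the reference.
; When that player begins overlapping the OverlapBox, it checks the PlayerColor enum and destroys itself immediately on a match.
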(event `self.ReceiveBeginPlay`
  (bind _asbp_player (cast `/Game/Blueprints/BP_player` (`GameplayStatics.GetPlayerCharacter` 0)))
  (set `self.PlayerRef` _asbp_player))

(event `self.OverlapBox.OnComponentBeginOverlap`
  (params (OverlappedComponent :type "PrimitiveComponent Object Reference") (OtherActor :type "Actor Object Reference") (OtherComp :type "PrimitiveComponent Object Reference") (OtherBodyIndex :type Integer) (bFromSweep :type Boolean) (SweepResult :type "HitResult Structure (by ref)"))
  (bind _playerref (`self.PlayerRef`))
  (if (== OtherActor _playerref)
    (if (`|EnumEquality` (`/Game/Blueprints/BP_player.PlayerColor` _playerref) "NewEnumerator2")
      (`self.K2_DestroyActor`))))

(fn `UserConstructionScript`)
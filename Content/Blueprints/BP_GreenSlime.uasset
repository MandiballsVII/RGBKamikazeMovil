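; BP_GreenSlime is a slime obstacle that responds to the player's color through an overlap box.
; When the player leaves the box in one color state, it switches once to a green block sprite, enables blocking-box collision and increments a collision counter.
; Once that counter is nonzero, the player entering the box in a second color state destroys the actor.
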(event `self.ReceiveBeginPlay`
  (bind _asbp_player (cast `/Game/Blueprints/BP_player` (`GameplayStatics.GetPlayerCharacter` 0)))
  (set `self.PlayerRef` _asbp_player))

(event `self.OverlapBox.OnComponentBeginOverlap`
  (params (OverlappedComponent :type "PrimitiveComponent Object Reference") (OtherActor :type "Actor Object Reference") (OtherComp :type "PrimitiveComponent Object Reference") (OtherBodyIndex :type Integer) (bFromSweep :type Boolean) (SweepResult :type "HitResult Structure (by ref)"))
  (bind _playerref (`self.PlayerRef`))
  (if (== OtherActor _playerref)
    (if (and (`|EnumEquality` (`/Game/Blueprints/BP_player.PlayerColor` _playerref) "NewEnumerator2") (!= (`self.NumberOfCollisions`) 0))
      (`self.K2_DestroyActor`))))

(event `self.OverlapBox.OnComponentEndOverlap`
  (params (OverlappedComponent :type "PrimitiveComponent Object Reference") (OtherActor :type "Actor Object Reference") (OtherComp :type "PrimitiveComponent Object Reference") (OtherBodyIndex :type Integer))
  (bind _playerref (`self.PlayerRef`))
  (if (== OtherActor _playerref)
    (if (== (`self.NumberOfCollisions`) 0)
      (if (`|EnumEquality` (`/Game/Blueprints/BP_player.PlayerColor` _playerref) "NewEnumerator1")
        (`PaperSpriteComponent.SetSprite` (`self.PaperSprite`) "/Game/PaperAssets/Objects/Sprites/Obstaculos_BloqueVerde_Sprite.Obstaculos_BloqueVerde_Sprite")
        (bind _result (`/Engine/EditorBlueprintResources/StandardMacros.IncrementInt` (`self.NumberOfCollisions`))
          (:`  `
            (set `self.NumberOfCollisions` _result)
            (`PrimitiveComponent.SetCollisionEnabled` (`self.CollisionBox`) "QueryAndPhysics")))))))

(fn `UserConstructionScript`)
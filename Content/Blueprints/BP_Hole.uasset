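; BP_Hole is a hazard that pulls the player in and restarts the current level.
; When the player hits the collision box, it briefly waits, disables that collision, and runs a timeline that lerps the player's XY toward the hole's center, keeping Z unchanged.
; After the timeline and another short delay, it reopens the current level by name.
; The player leaving the inner overlap box re-enables the collision.
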(event `self.ReceiveBeginPlay`
  (bind _asbp_player (cast `/Game/Blueprints/BP_player` (`GameplayStatics.GetPlayerCharacter` 0)))
  (set `self.PlayerRef` _asbp_player))

(event `self.CollsionBox.OnComponentHit`
  (params (HitComponent :type "PrimitiveComponent Object Reference") (OtherActor :type "Actor Object Reference") (OtherComp :type "PrimitiveComponent Object Reference") (NormalImpulse :type "Vector Structure") (Hit :type "HitResult Structure (by ref)"))
  (bind (_returnvalue_x _returnvalue_y) (`KismetMathLibrary.BreakVector` (`self.K2_GetActorLocation`)))
  (bind (_returnvalue_x_2 _returnvalue_y_2 _returnvalue_z) (`KismetMathLibrary.BreakVector` (`self.K2_GetActorLocation` (`self.PlayerRef`))))
  (if (== OtherActor (`self.PlayerRef`))
    (`KismetSystemLibrary.Delay` 0.2)
    (`PrimitiveComponent.SetCollisionEnabled` (`self.CollsionBox`) "NoCollision")
    (bind (_direction _transport) (`Timeline|TransportPlayer` :!via `PlayFromStart`)
      (:`Update`
        (`self.K2_SetActorLocation` (`self.PlayerRef`) (`KismetMathLibrary.MakeVector` (`KismetMathLibrary.Lerp` _returnvalue_x_2 _returnvalue_x _transport) (`KismetMathLibrary.Lerp` _returnvalue_y_2 _returnvalue_y _transport) _returnvalue_z) false false))
      (:`Finished`
        (`KismetSystemLibrary.Delay` 0.2)
        (bind _returnvalue (`GameplayStatics.GetCurrentLevelName` true))
        (`GameplayStatics.OpenLevel` (`KismetStringLibrary.Conv_StringToName` _returnvalue))))))

(event `self.InsideOverlapBox.OnComponentEndOverlap`
  (params (OverlappedComponent :type "PrimitiveComponent Object Reference") (OtherActor :type "Actor Object Reference") (OtherComp :type "PrimitiveComponent Object Reference") (OtherBodyIndex :type Integer))
  (if (== OtherActor (`self.PlayerRef`))
    (`PrimitiveComponent.SetCollisionEnabled` (`self.CollsionBox`) "QueryAndPhysics")))

(fn `UserConstructionScript`)
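; BP_LevelNumberText is an actor that displays the current level number in the world through a TextRender component.
; On BeginPlay it caches a reference to BP_GameInstance, then calls ChangeText to set the text to "Level:" plus the instance's LevelNumber.
; The label is set at start and only changes again if ChangeText is called.
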(event `self.ReceiveBeginPlay`
  (bind _asbp_game_instance (cast `/Game/Blueprints/BP_GameInstance` (`GameplayStatics.GetGameInstance`)))
  (set `self.GameInstanceRef` _asbp_game_instance)
  (`self.ChangeText`))

(event `ChangeText`
  (`TextRenderComponent.K2_SetText` (`self.TextRender`) (`KismetTextLibrary.Conv_StringToText` (`KismetStringLibrary.Concat_StrStr` "Level: " (`KismetStringLibrary.Conv_IntToString` (`/Game/Blueprints/BP_GameInstance.LevelNumber` (`self.GameInstanceRef`)))))))

(fn `UserConstructionScript`)
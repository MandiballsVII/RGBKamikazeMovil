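; BP_Rack is an actor that lets the player pass into it only when their color matches one specific enum value.
; A matching hit disables the collision box after a short delay, then a timeline lerps the player to the rack's XY with sweep, keeping Z.
; The player's moving flag clears when the timeline finishes, or immediately for other colors.
; Ending overlap with the inner box re-enables collision.
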(event `self.ReceiveBeginPlay`
  (bind _asbp_player (cast `/Game/Blueprints/BP_player` (`GameplayStatics.GetPlayerCharacter` 0)))
  (bind _output_get (set `self.PlayerRef` _asbp_player)))

(event `self.CollsionBox.OnComponentHit`
  (params (HitComponent :type "PrimitiveComponent Object Reference") (OtherActor :type "Actor Object Reference") (OtherComp :type "PrimitiveComponent Object Reference") (NormalImpulse :type "Vector Structure") (Hit :type "HitResult Structure (by ref)"))
  (bind (_returnvalue_x _returnvalue_y) (`KismetMathLibrary.BreakVector` (`self.K2_GetActorLocation`)))
  (bind _playerref (`self.PlayerRef`))
  (bind _playerref_2 (`self.PlayerRef`))
  (bind (_returnvalue_x_2 _returnvalue_y_2 _returnvalue_z) (`KismetMathLibrary.BreakVector` (`self.K2_GetActorLocation` (`self.PlayerRef`))))
  (if (== OtherActor _playerref)
    (if (`|EnumEquality` (`/Game/Blueprints/BP_player.PlayerColor` _playerref) "NewEnumerator3")
      (`KismetSystemLibrary.Delay` 0.2)
      (`PrimitiveComponent.SetCollisionEnabled` (`self.CollsionBox`) "NoCollision")
      (bind (_direction _transport) (`Timeline|TransportPlayer` :!via `PlayFromStart`)
        (:`Update`
          (`self.K2_SetActorLocation` _playerref_2 (`KismetMathLibrary.MakeVector` (`KismetMathLibrary.Lerp` _returnvalue_x_2 _returnvalue_x _transport) (`KismetMathLibrary.Lerp` _returnvalue_y_2 _returnvalue_y _transport) _returnvalue_z) true false))
        (:`Finished`
          (set `/Game/Blueprints/BP_player.IsMoving` false _playerref_2)))
      (else
        (set `/Game/Blueprints/BP_player.IsMoving` false (stale `self.ReceiveBeginPlay` _output_get))))))

(event `self.InsideOverlapBox.OnComponentEndOverlap`
  (params (OverlappedComponent :type "PrimitiveComponent Object Reference") (OtherActor :type "Actor Object Reference") (OtherComp :type "PrimitiveComponent Object Reference") (OtherBodyIndex :type Integer))
  (if (== OtherActor (`self.PlayerRef`))
    (`PrimitiveComponent.SetCollisionEnabled` (`self.CollsionBox`) "QueryAndPhysics")))

(fn `UserConstructionScript`)
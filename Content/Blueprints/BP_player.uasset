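; Player pawn for a level-based sliding game, moving along X or Y until it hits something.
; Axis input starts looping timers that apply swept, accelerating moves and block new input while moving.
; Capsule hits clear the timers, snap position to whole units, handle hole and rack tags, and advance the GameInstance level at the finish.
; It also cycles level-unlocked flipbook colors, periodically wiggles when red, and opens the pause menu.
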(event `self.ReceiveBeginPlay`
  (`PrimitiveComponent.SetSimulatePhysics` (`self.CapsuleComponent`) false)
  (bind _asbp_game_instance (cast `/Game/Blueprints/BP_GameInstance` (`GameplayStatics.GetGameInstance`)))
  (set `self.GameInstanceRef` _asbp_game_instance)
  (`KismetSystemLibrary.K2_SetTimerDelegate` (delegate `Tremble`) (`KismetMathLibrary.Conv_IntToDouble` (`KismetMathLibrary.RandomIntegerInRange` 5 10)) true))

(event `Tremble`
  (bind _sprite (`self.Sprite`))
  (if (`|EnumEquality` (`self.PlayerColor`) "NewEnumerator2")
    (`PaperFlipbookComponent.SetFlipbook` _sprite "/Game/PaperAssets/Character/Flipbooks/FB_RedWiggle.FB_RedWiggle")
    (`KismetSystemLibrary.Delay` 0.3)
    (`PaperFlipbookComponent.SetFlipbook` _sprite "/Game/PaperAssets/Character/Flipbooks/FB_RedIdle.FB_RedIdle")))

(event `self.CapsuleComponent.OnComponentHit`
  (params (HitComponent :type "PrimitiveComponent Object Reference") (OtherActor :type "Actor Object Reference") (OtherComp :type "PrimitiveComponent Object Reference") (NormalImpulse :type "Vector Structure") (Hit :type "HitResult Structure (by ref)"))
  ;[1 0.4902 0.4902] Character Movement
  (`KismetSystemLibrary.K2_ClearAndInvalidateTimerHandle` (stale `InputAxis|X_Axis` _returnvalue))
  (`KismetSystemLibrary.K2_ClearAndInvalidateTimerHandle` (stale `InputAxis|X_Axis` _returnvalue_2))
  (`KismetSystemLibrary.K2_ClearAndInvalidateTimerHandle` (stale `InputAxis|X_Axis` _returnvalue_3))
  (`KismetSystemLibrary.K2_ClearAndInvalidateTimerHandle` (stale `InputAxis|X_Axis` _returnvalue_4))
  (set `self.PlayerSpeed` (0.0 0.0 0.0))
  (`KismetSystemLibrary.Delay` 0.1)
  (`self.RelocatePlayer`)
  (if (`BlueprintGameplayTagLibrary.HasTag` (`self.GameplayTags`) (struct :`TagName` "Location.InFinish"))
    (`self.RelocatePlayer`)
    (`KismetSystemLibrary.Delay` 0.2)
    (`/Game/Blueprints/BP_GameInstance.IncrementLevelNumber` (`self.GameInstanceRef`))
    (`KismetSystemLibrary.Delay` 1.0)
    (set `self.IsMoving` false :!label _label)
    (elif (`self.ActorHasTag` OtherActor "Hole")
      (`KismetSystemLibrary.Delay` 1.7)
      (goto _label)
      (elif (not (`self.ActorHasTag` OtherActor "Rack"))
        (`self.RelocatePlayer`)
        (goto _label)))))

(event `MoveRight`
  ;[1 0.4902 0.4902] Character Movement
  (`self.MovePlayerToPositive`)
  (`self.AccelerationX`))

(event `InputAxis|X_Axis`
  (params (AxisValue :type "Float (single-precision)"))
  ;[1 0.4902 0.4902] Character Movement
  (if (`self.IsMoving`) :!label _label_2
    _
    (elif (> AxisValue 0.0)
      (set `self.IsMoving` true)
      (bind _returnvalue (`KismetSystemLibrary.K2_SetTimerDelegate` (delegate `MoveRight`) (`self.MovementTimerSpeed`) true))
      (elif (< AxisValue 0.0)
        (set `self.IsMoving` true)
        (bind _returnvalue_2 (`KismetSystemLibrary.K2_SetTimerDelegate` (delegate `MoveLeft`) (`self.MovementTimerSpeed`) true))
        (elif (> (stale `InputAxis|Y_Axis` AxisValue) 0.0)
          (set `self.IsMoving` true)
          (bind _returnvalue_3 (`KismetSystemLibrary.K2_SetTimerDelegate` (delegate `MoveUp`) (`self.MovementTimerSpeed`) true))
          (elif (< (stale `InputAxis|Y_Axis` AxisValue) 0.0)
            (set `self.IsMoving` true)
            (bind _returnvalue_4 (`KismetSystemLibrary.K2_SetTimerDelegate` (delegate `MoveDown`) (`self.MovementTimerSpeed`) true))))))))

(event `InputAxis|Y_Axis`
  (params (AxisValue :type "Float (single-precision)"))
  ;[1 0.4902 0.4902] Character Movement
  (goto _label_2))

(event `MoveLeft`
  ;[1 0.4902 0.4902] Character Movement
  (`self.MovePlayerToNegative`)
  (`self.AccelerationX`))

(event `MoveUp`
  ;[1 0.4902 0.4902] Character Movement
  (`self.MovePlayerToNegative`)
  (`self.AccelerationY`))

(event `MoveDown`
  ;[1 0.4902 0.4902] Character Movement
  (`self.MovePlayerToPositive`)
  (`self.AccelerationY`))

(event `InputAction|ChangeColor`
  (params (Key :type "Key Structure"))
  (bind _sprite (`self.Sprite`))
  (bind _levelnumber (`/Game/Blueprints/BP_GameInstance.LevelNumber` (`self.GameInstanceRef`)))
  ;[1 0.4902 0.4902] Color Change
  (:`Pressed`
    (switch `/Game/Enums/E_PlayerColor` (`self.PlayerColor`)
      (:`NewEnumerator0`
        (if (> _levelnumber 10)
          (`PaperFlipbookComponent.SetFlipbook` _sprite "/Game/PaperAssets/Character/Flipbooks/FB_GreenIdle.FB_GreenIdle")
          (set `self.PlayerColor` "NewEnumerator1")))
      (:`NewEnumerator1`
        (if (> _levelnumber 20)
          (`PaperFlipbookComponent.SetFlipbook` _sprite "/Game/PaperAssets/Character/Flipbooks/FB_RedIdle.FB_RedIdle")
          (set `self.PlayerColor` "NewEnumerator2")
          (else
            (`PaperFlipbookComponent.SetFlipbook` _sprite "/Game/PaperAssets/Character/Flipbooks/FB_Grey.FB_Grey" :!label _label_3)
            (set `self.PlayerColor` "NewEnumerator0"))))
      (:`NewEnumerator2`
        (if (> _levelnumber 30)
          (`PaperFlipbookComponent.SetFlipbook` _sprite "/Game/PaperAssets/Character/Flipbooks/FB_BlueIdle.FB_BlueIdle")
          (set `self.PlayerColor` "NewEnumerator3")
          (else
            (goto _label_3))))
      (:`NewEnumerator3`
        (goto _label_3)))))

(event `InputAction|Pause`
  (params (Key :type "Key Structure"))
  (bind _returnvalue (`GameplayStatics.GetPlayerController` 0))
  ;[0.4106 1 0.572] Pause
  (:`Pressed`
    (if (not (`self.Paused`))
      (`GameplayStatics.SetGamePaused` true)
      (bind _returnvalue_2 (`|CreateWidget` "/Game/UI/PauseMenu.PauseMenu_C" _returnvalue))
      (`UserWidget.AddToViewport` _returnvalue_2 0)
      (`WidgetBlueprintLibrary.SetInputMode_GameAndUIEx` _returnvalue _returnvalue_2)
      (set `self.Paused` true)
      (set `PlayerController.bShowMouseCursor` true _returnvalue))))

(fn `AccelerationX`
  (bind _playerspeed_x (`KismetMathLibrary.BreakVector` (`self.PlayerSpeed`)))
  (if (< _playerspeed_x 1.0)
    (set `self.PlayerSpeed` (`KismetMathLibrary.MakeVector` (+ _playerspeed_x 0.001)))))

(fn `AccelerationY`
  (bind (_playerspeed_x _playerspeed_y) (`KismetMathLibrary.BreakVector` (`self.PlayerSpeed`)))
  (if (< _playerspeed_y 1.0)
    (set `self.PlayerSpeed` (`KismetMathLibrary.MakeVector` 0.0 (+ _playerspeed_y 0.001)))))

(fn `MovePlayerToNegative`
  (`self.K2_SetActorLocation` (- (`self.K2_GetActorLocation`) (`self.PlayerSpeed`)) true))

(fn `MovePlayerToPositive`
  (`self.K2_SetActorLocation` (+ (`self.K2_GetActorLocation`) (`self.PlayerSpeed`)) true))

(fn `RelocatePlayer`
  (bind (_returnvalue_x _returnvalue_y) (`KismetMathLibrary.BreakVector` (`self.K2_GetActorLocation`)))
  (`self.K2_SetActorLocation` (`KismetMathLibrary.MakeVector` (`KismetMathLibrary.Conv_IntToDouble` (`KismetMathLibrary.Round` _returnvalue_x)) (`KismetMathLibrary.Conv_IntToDouble` (`KismetMathLibrary.Round` _returnvalue_y)) 36.150002)))

(fn `UserConstructionScript`)